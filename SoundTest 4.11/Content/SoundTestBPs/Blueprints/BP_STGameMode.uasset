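; Game mode for a sound visualizer test that moves cubes in the level to the frequency spectrum of a selected song.
; On BeginPlay it gathers seven cube groups and loads .ogg files from a platform-dependent hard-coded folder, chaining each load completion into a UI button and the next load.
; SoundVisComponent handles play, pause and stop, and its spectrum callback sets each group's height from its band's average, scaled by a hand-tuned range.
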(event OnFileLoadCompleted(SoundVisComponent)
  (params (SoundWaveRef :type Sound%20Wave%20Object%20Reference))
  (bind _soundlistwidgetref (Variables|Default|GetSoundListWidgetRef))
  ;[1 1 1] When loading finished, add a new button to the SoundList Widget and try to get the next SoundFile
  (Utilities|IsValid _soundlistwidgetref
    (:Is%20Valid
      (Default|CreateNewSoundButton _soundlistwidgetref SoundWaveRef (Utilities|Text|ToText(String) (Utilities|Array|Get(acopy) (Variables|Default|GetCurrentSoundFileNames) (Variables|Default|GetCurrentSoundNameIndex))) (Variables|Default|GetCurrentSoundNameIndex))
      (Math|Integer|IncrementInt (Variables|Default|GetCurrentSoundNameIndex)
        (:%20%20
          (CallFunction|LoadNextSoundFile))))))

(event OnFrequencySpectrumCalculated(SoundVisComponent)
  (params (OutFrequencies :type Array%20of%20Floats%20%28single-precision%29))
  ;[1 1 1] This gets called every 0.01 seconds from C++ when you have the automated "Start.." event called
  (Variables|Default|SetCurrentFrequencies OutFrequencies)
  (Utilities|FlowControl|Sequence
    (:then_0
      ;[1 1 1] This is controlling the Height of the Blocks based on the Average Frew Value
      ;;[1 0 0] "MaxRange" needs to be adjusted based on the  sound you play
      (Default|AdjustHeight (Variables|Default|GetSubBassCubes) (Class|SoundVisComponent|GetAverageFrequencyValueinRange (Variables|Default|GetCurrentSound) (Variables|Default|GetCurrentFrequencies) 20 60) 9e+05))
    (:then_1
      (Default|AdjustHeight (Variables|Default|GetBassCubes) (Class|SoundVisComponent|GetAverageFrequencyValueinRange (Variables|Default|GetCurrentSound) (Variables|Default|GetCurrentFrequencies) 60 250) 5e+05))
    (:then_2
      (Default|AdjustHeight (Variables|Default|GetLowMidCubes) (Class|SoundVisComponent|GetAverageFrequencyValueinRange (Variables|Default|GetCurrentSound) (Variables|Default|GetCurrentFrequencies) 250 500) 2e+05))
    (:then_3
      (Default|AdjustHeight (Variables|Default|GetMidCubes) (Class|SoundVisComponent|GetAverageFrequencyValueinRange (Variables|Default|GetCurrentSound) (Variables|Default|GetCurrentFrequencies) 500 2000) 8e+04))
    (:then_4
      (Default|AdjustHeight (Variables|Default|GetHighMidCubes) (Class|SoundVisComponent|GetAverageFrequencyValueinRange (Variables|Default|GetCurrentSound) (Variables|Default|GetCurrentFrequencies) 2000 4000) 5e+04))
    (:then_5
      (Default|AdjustHeight (Variables|Default|GetPresenceCubes) (Class|SoundVisComponent|GetAverageFrequencyValueinRange (Variables|Default|GetCurrentSound) (Variables|Default|GetCurrentFrequencies) 4000 6000) 3.5e+04))
    (:then_6
      (Default|AdjustHeight (Variables|Default|GetBrillianceCubes) (Class|SoundVisComponent|GetAverageFrequencyValueinRange (Variables|Default|GetCurrentSound) (Variables|Default|GetCurrentFrequencies) 6000 16000) 1.5e+04))))

(event Custom|StopSound
  ;[1 1 1] Event manages Pausing, Resuming and Playing a Sound
  ;;[1 1 1] Event manages Stopping a Sound
  (Class|SoundVisComponent|StopCalculatingFrequencySpectrum (Variables|Default|GetSoundVisComponent)))

(event Custom|LoadSoundFileNames
  (bind _soundviscomponent (Variables|Default|GetSoundVisComponent))
  ;[1 1 0] ADJUST THIS TO LOAD YOUR OWN SOUNDS! Load the SoundFile Names and save them in an Array
  ;;[1 1 1] Note: This branching pattern can be useful for debugging android projects on PC/Mac/Linux
  (bind _returnvalue (Game|GetPlatformName))
  (if (Utilities|Enum|Equal(Enum) _returnvalue "Android")
    (bind (_bloaded _outsoundfilenameswithpath _outsoundfilenameswithoutpath) (Class|SoundVisComponent|LoadAllSoundFileNamesfromHD _soundviscomponent "/sdcard/Songs/" true "ogg"))
    (if _bloaded
      (Variables|Default|SetCurrentSoundFilePaths _outsoundfilenameswithpath)
      (Variables|Default|SetCurrentSoundFileNames _outsoundfilenameswithoutpath))
    (else
      (bind (_bloaded_2 _outsoundfilenameswithpath_2 _outsoundfilenameswithoutpath_2) (Class|SoundVisComponent|LoadAllSoundFileNamesfromHD _soundviscomponent "/Users/micador/Sourcetree/GoogleSoundVis/SoundTest 4.11/Songs/" true "ogg")) ; Please note: only absolute paths are currently working for the Android platform.
      (if _bloaded_2
        (Variables|Default|SetCurrentSoundFilePaths _outsoundfilenameswithpath_2)
        (Variables|Default|SetCurrentSoundFileNames _outsoundfilenameswithoutpath_2)))))

(event Custom|LoadNextSoundFile
  ;[1 1 1] Try to load the next SoundFile
  (if (Math|Boolean|ANDBoolean (< (Variables|Default|GetCurrentSoundNameIndex) (Variables|Default|GetMaxNumberOfSoundsToLoad)) (>= (Variables|Default|GetCurrentSoundNameIndex) 0) (< (Variables|Default|GetCurrentSoundNameIndex) (Utilities|Array|Length (Variables|Default|GetCurrentSoundFilePaths))))
    (Class|SoundVisComponent|LoadSoundFilefromHD (Variables|Default|GetSoundVisComponent) (Utilities|Array|Get(acopy) (Variables|Default|GetCurrentSoundFilePaths) (Variables|Default|GetCurrentSoundNameIndex)))))

(event Custom|SetupUI
  ;[1 1 1] Setup UI
  (bind _returnvalue (UserInterface|CreateWidget "/Game/SoundTestBPs/Widgets/SoundListWidget.SoundListWidget_C"))
  (bind _output_get (Variables|Default|SetSoundListWidgetRef _returnvalue))
  (UserInterface|Viewport|AddtoViewport _output_get 0)
  (Input|SetInputModeGameandUI (Game|GetPlayerController 0) 0 true false)
  (Variables|/Script/Engine.PlayerController|SetbShowMouseCursor (Game|GetPlayerController 0) true))

(event Custom|ToggleSound
  (params (InSoundWave :type Sound%20Wave%20Object%20Reference))
  ;[1 1 1] Event manages Pausing, Resuming and Playing a Sound
  (Variables|Default|SetCurrentSound InSoundWave)
  (if (Class|SoundVisComponent|IsPlayerPlaying (Variables|Default|GetSoundVisComponent))
    (Class|SoundVisComponent|PauseCalculatingFrequencySpectrum (Variables|Default|GetSoundVisComponent))
    (elif (Class|SoundVisComponent|IsPlayerPaused (Variables|Default|GetSoundVisComponent))
      (Class|SoundVisComponent|ResumeCalculatingFrequencySpectrum (Variables|Default|GetSoundVisComponent))
      (else
        ;;[1 0 0] Segment Length of 0.1 means, we analyze 0.1 sec of the sound, giving us around 4100 samples for a sound with 44100 samplerate
        (Class|SoundVisComponent|StartCalculatingFrequencySpectrum (Variables|Default|GetSoundVisComponent) (Variables|Default|GetCurrentSound) 0.1)))))

(event Custom|GetAllCubes
  ;[1 1 1] Get Bass, Mid and High Frequency Cubes that we want to move with the actual Frequency Spectrum
  (Utilities|FlowControl|Sequence
    (:then_0
      (bind _outactors (Actor|GetAllActorsOfClass "/Game/SoundTestBPs/Blueprints/Cubes/SubBassCube.SubBassCube_C"))
      (Variables|Default|SetSubBassCubes _outactors)
      (bind _outactors_2 (Actor|GetAllActorsOfClass "/Game/SoundTestBPs/Blueprints/Cubes/BassCube.BassCube_C"))
      (Variables|Default|SetBassCubes _outactors_2))
    (:then_1
      (bind _outactors_3 (Actor|GetAllActorsOfClass "/Game/SoundTestBPs/Blueprints/Cubes/LowMidCube.LowMidCube_C"))
      (Variables|Default|SetLowMidCubes _outactors_3)
      (bind _outactors_4 (Actor|GetAllActorsOfClass "/Game/SoundTestBPs/Blueprints/Cubes/MidCub.MidCub_C"))
      (Variables|Default|SetMidCubes _outactors_4)
      (bind _outactors_5 (Actor|GetAllActorsOfClass "/Game/SoundTestBPs/Blueprints/Cubes/HighMidCube.HighMidCube_C"))
      (Variables|Default|SetHighMidCubes _outactors_5))
    (:then_2
      (bind _outactors_6 (Actor|GetAllActorsOfClass "/Game/SoundTestBPs/Blueprints/Cubes/PresenceCube.PresenceCube_C"))
      (Variables|Default|SetPresenceCubes _outactors_6)
      (bind _outactors_7 (Actor|GetAllActorsOfClass "/Game/SoundTestBPs/Blueprints/Cubes/BrillianceCube.BrillianceCube_C"))
      (Variables|Default|SetBrillianceCubes _outactors_7))))

(event EventBeginPlay
  ;[1 1 1] Just setting up some stuff, like UI, or getting references to all the Blocks in our level
  (CallFunction|SetupUI)
  (CallFunction|GetAllCubes)
  (CallFunction|LoadSoundFileNames)
  (CallFunction|LoadNextSoundFile))

(fn ConstructionScript)